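; Food placement manager that hands out table placement waypoints and tracks which are taken, with reset logic named for AI use.
; A boolean tracker array runs parallel to the waypoint array: GetNextWaypoint claims the first free entry and returns that waypoint with its index.
; ResetAiWaypoint frees a claimed entry by index, and both functions print debug messages.
; The event graph and construction script are empty.
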(event `self.ReceiveBeginPlay`)

(fn `GetNextWaypoint`
  (returns (NextAvablieTableplacement :type "/Game/Blueprints/TablePlaement Object Reference") (waypointIndex :type Integer))
  (bind _waypointtracker (`self.WaypointTracker`))
  (for _index (range (`KismetArrayLibrary.Array_Length` _waypointtracker))
    (if (not (`|GetArrayItem` _waypointtracker _index))
      (`KismetSystemLibrary.PrintString` (`KismetStringLibrary.BuildString_Int` "" "Foundwaypoint: " _index) true true (struct :`G` 0.66 :`B` 1.0 :`A` 1.0) 100.0)
      (`KismetArrayLibrary.Array_Set` _waypointtracker _index true)
      (return (`|GetArrayItem` (`self.Waypoints`) _index) _index))))

(fn `ResetAiWaypoint`
  (params (NewParam :type Integer))
  (bind _waypointtracker (`self.WaypointTracker`))
  (if (`|GetArrayItem` _waypointtracker NewParam)
    (`KismetSystemLibrary.PrintString` (`KismetStringLibrary.BuildString_Int` "" "Resetwaypoint: " NewParam))
    (`KismetArrayLibrary.Array_Set` _waypointtracker NewParam)
    (return)))

(fn `UserConstructionScript`)