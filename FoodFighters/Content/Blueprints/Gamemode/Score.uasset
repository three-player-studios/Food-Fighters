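; Score is a match countdown Blueprint that also starts the game's audio.
; BeginPlay plays uplifted music and crowd ambiance as 2D sounds.
; Tick uses a one-second Delay to step down seconds, rolling over into minutes, and prints a time-over message when both reach zero.
; Nothing halts the countdown at zero, and the Set Game Paused node is left unconnected.
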(event `self.ReceiveTick`
  (params (DeltaSeconds :type "Float (single-precision)"))
  (`|ExecutionSequence`
    (:`then_0`
      (`KismetSystemLibrary.Delay` 1.0)
      (set `self.Sec` (- (`self.Sec`) 1))
      (if (< (`self.Sec`) 0)
        (set `self.Minutes` (- (`self.Minutes`) 1))
        (set `self.Sec` 59))
      (if (== (`self.Sec`) 0)
        (if (== (`self.Minutes`) 0)
          (`KismetSystemLibrary.PrintString` "Kicten time Over"))))))

(event `self.ReceiveBeginPlay`
  (`|ExecutionSequence`
    (:`then_0`
      (`GameplayStatics.PlaySound2D` "/Game/Sound/uplifted_music.uplifted_music"))
    (:`then_1`
      (`GameplayStatics.PlaySound2D` "/Game/Sound/crowd_ambiance.crowd_ambiance"))))

(fn `UserConstructionScript`)