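; BP_Test_Oven_Interact is a test interactable, named as an oven, that opens a UI widget when the player interacts with it.
; On BeginPlay it creates a UMG_TEST_INTERACT widget and caches the player character cast to PlayerReal.
; The ObjectInteract event adds that pre-built widget to the viewport, prints a debug string and calls EndInput on the cached player.
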(event `self.ReceiveTick`
  (params (DeltaSeconds :type "Float (single-precision)")))

(event `self.ReceiveBeginPlay`
  (bind _returnvalue (`|CreateWidget` "/Game/UMG/UMG_TEST_INTERACT.UMG_TEST_INTERACT_C"))
  (set `self.UI_Widget` _returnvalue)
  (bind _asplayer_real (cast `/Game/Blueprints/Charater/PlayerReal` (`GameplayStatics.GetPlayerCharacter` 0)))
  (set `self.NewVar_1` _asplayer_real))

(event `/Game/Blueprints/Interaction/I_Interact.Object_Interact`
  (`UserWidget.AddToViewport` (`self.UI_Widget`) 0)
  (`KismetSystemLibrary.PrintString` "fart")
  (`/Game/Blueprints/Charater/PlayerReal.EndInput` (`self.NewVar_1`)))

(fn `UserConstructionScript`)