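; BP_Stove is an interactable cooking stove that, on interaction, ends player input and opens a UMG_Stove widget linked to itself.
; Helper functions snap food to the "Inside" socket of either the pot or stove mesh.
; Every tick, cook and boil functions write to the same StoveTimer progress slider, boil last.
; The boil percentage divides BoilCurrentTime by itself rather than by a total.
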(event `/Game/Blueprints/Interaction/I_Interact.Object_Interact`
  (bind _asplayer_real (cast `/Game/Blueprints/Charater/PlayerReal` (`GameplayStatics.GetPlayerCharacter` 0)))
  (`/Game/Blueprints/Charater/PlayerReal.EndInput` _asplayer_real)
  (bind _returnvalue (`|CreateWidget` "/Game/UMG/Food/UMG_Stove.UMG_Stove_C"))
  (`/Game/UMG/Food/UMG_Stove.GetStove` _returnvalue self)
  (`UserWidget.AddToViewport` _returnvalue 0))

(event `self.ReceiveTick`
  (params (DeltaSeconds :type "Float (single-precision)"))
  (`self.CookTimer`)
  (`self.BoilTimer`))

(fn `BoilTimer`
  (bind _asstove_timer (cast `/Game/UMG/StoveTimer` (`WidgetComponent.GetUserWidgetObject` (`self.StoveTimer`))))
  (`ProgressBar.SetPercent` (`/Game/UMG/StoveTimer.ProgressSlider` _asstove_timer) (/ (`self.BoilCurrentTime`) (`self.BoilCurrentTime`))))

(fn `CookTimer`
  (bind _asstove_timer (cast `/Game/UMG/StoveTimer` (`WidgetComponent.GetUserWidgetObject` (`self.StoveTimer`))))
  (`ProgressBar.SetPercent` (`/Game/UMG/StoveTimer.ProgressSlider` _asstove_timer) (/ (`self.CookCurrentTime`) (`self.CookTotalTime`))))

(fn `PlaceItemInPot`
  (params (Food :type "Food Object Reference"))
  (`self.K2_AttachToComponent` Food (`self.PotMesh`) "Inside" "SnapToTarget" "KeepWorld" "KeepWorld" true))

(fn `PlaceItemInStove`
  (params (Food :type "Food Object Reference"))
  (`self.K2_AttachToComponent` Food (`self.StoveMesh`) "Inside" "SnapToTarget" "KeepWorld" "KeepWorld" true))

(fn `UserConstructionScript`)