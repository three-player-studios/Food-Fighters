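; BP_CuttingBoard is an interactable cutting board intended for cutting the player's held food.
; ObjectInteract checks the player's HeldFood, printing a message if none is held, otherwise disabling input and setting a Cutting flag.
; Tick increments a frame counter without checking that flag and re-enables player input when it exactly equals CutTotalTime.
; The counter never resets, and the food itself is not modified here.
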(event `/Game/Blueprints/Interaction/I_Interact.Object_Interact`
  (bind _asplayer_real (cast `/Game/Blueprints/Charater/PlayerReal` (`GameplayStatics.GetPlayerCharacter` 0)))
  (if (`KismetStringLibrary.EqualEqual_StrStr` (`Food.Name` (`/Game/Blueprints/Charater/PlayerReal.HeldFood` _asplayer_real)))
    (`KismetSystemLibrary.PrintString` "No Food To Cut")
    (else
      (`self.DisableInput` _asplayer_real null)
      (set `self.Cutting` true))))

(event `self.ReceiveTick`
  (params (DeltaSeconds :type "Float (single-precision)"))
  (bind _output_get (set `self.CutCurrentTime` (+ (`self.CutCurrentTime`) 1)))
  (if (== _output_get (`self.CutTotalTime`))
    (bind _asplayer_real (cast `/Game/Blueprints/Charater/PlayerReal` (`GameplayStatics.GetPlayerCharacter` 0)))
    (`self.EnableInput` _asplayer_real null)))

(fn `UserConstructionScript`)