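; Restaurant customer NPC that claims a table waypoint from the FoodPlacementManager, walks there and sits facing by seat index.
; Food is checked only on arrival; if present with time remaining, it walks to checkout, awards PlayerReal points, then exits.
; Tick counts down a wait timer shown on a widget progress bar; at zero the NPC heads for the exit.
; Movement chains AIMoveTo and montages, freeing the waypoint before destruction.
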(event `self.ReceiveBeginPlay`
  (bind _tableplacementmanger (`self.TablePlacementManger`))
  ;[1 1 1] Comment
  (`KismetSystemLibrary.Delay` 2.0)
  (`KismetSystemLibrary.PrintString` "Spawn IN" true true (struct :`G` 0.66 :`B` 1.0 :`A` 1.0) 100.0)
  (bind _asfood_placement_manager (cast `/Game/Blueprints/FoodPlacementManager` _tableplacementmanger)
    (:`then`
      (`KismetSystemLibrary.PrintString` "sUccess Table found" true true (struct :`G` 0.66 :`B` 1.0 :`A` 1.0) 100.0)
      (set `self.DestinationManager` _asfood_placement_manager)
      (`self.Move` self))
    (:`CastFailed`
      (`KismetSystemLibrary.PrintString` "FAIL to find table" true true (struct :`G` 0.66 :`B` 1.0 :`A` 1.0) 100.0)
      (`/Engine/EditorBlueprintResources/StandardMacros.IsValid` _tableplacementmanger
        (:`Is Valid`
          (`KismetSystemLibrary.PrintString` "Valid" true true (struct :`G` 0.66 :`B` 1.0 :`A` 1.0) 100.0))
        (:`Is Not Valid`
          (`KismetSystemLibrary.PrintString` "Not Valid" true true (struct :`G` 0.66 :`B` 1.0 :`A` 1.0) 100.0))))))

(event `self.ReceiveTick`
  (params (DeltaSeconds :type "Float (single-precision)"))
  (`|ExecutionSequence`
    (:`then_0`
      (`self.TIMENPC` self)
      (if (<= (`self.CurTime `) 0.0)
        (if (not (`self.ai cycle ended`))
          ;[1 1 1] Comment
          (set `self.ai cycle ended` true)
          (bind _returnvalue (`self.PlayAnimMontage` "/Game/Blueprints/Charater/standup.standup"))
          (`KismetSystemLibrary.Delay` _returnvalue)
          (`AITask_MoveTo.AIMoveTo` (`AIBlueprintHelperLibrary.GetAIController` self) (`KismetMathLibrary.MakeVector` (.x (`SceneComponent.K2_GetComponentLocation` (`Actor.RootComponent` (`/Game/Blueprints/FoodPlacementManager.Exit` (`self.DestinationManager`))))) (.y (`SceneComponent.K2_GetComponentLocation` (`Actor.RootComponent` (`/Game/Blueprints/FoodPlacementManager.Exit` (`self.DestinationManager`)))))) null -1.0 "Default" "Default" true false true
            (:`OnRequestFailed`
              (`KismetSystemLibrary.PrintString` "NPC did not move "))
            (:`OnMoveFinished`
              (`KismetSystemLibrary.PrintString` "NPC has Exit")
              ;[1 1 1] Comment
              (`/Game/Blueprints/FoodPlacementManager.ResetAiWaypoint` (`self.DestinationManager`) (`self.indexwaypoints`))
              (`KismetSystemLibrary.PrintString` (`KismetStringLibrary.Conv_IntToString` (`self.indexwaypoints`)) false true (struct :`G` 0.66 :`B` 1.0 :`A` 1.0) 100.0)
              (`KismetSystemLibrary.PrintString` "Resthappen" false true (struct :`G` 0.66 :`B` 1.0 :`A` 1.0) 100.0)
              (`self.K2_DestroyActor` self)
              (if true
                (`KismetSystemLibrary.PrintString` "FOOD IS IS ON TABLE ")
                (if (not (`self.Ai _pay_cycle`))
                  (set `self.Ai _pay_cycle` true)
                  (bind _returnvalue_2 (`self.PlayAnimMontage` "/Game/Blueprints/Charater/standup.standup"))
                  (`KismetSystemLibrary.Delay` _returnvalue_2)
                  (`AITask_MoveTo.AIMoveTo` (`AIBlueprintHelperLibrary.GetAIController` self) (`KismetMathLibrary.MakeVector` (.x (`SceneComponent.K2_GetComponentLocation` (`Actor.RootComponent` (`/Game/Blueprints/FoodPlacementManager.Checkout` (`self.DestinationManager`))))) (.y (`SceneComponent.K2_GetComponentLocation` (`Actor.RootComponent` (`/Game/Blueprints/FoodPlacementManager.Checkout` (`self.DestinationManager`)))))) null 0.1 "Default" "Default" true false true
                    (:`OnRequestFailed`
                      (`KismetSystemLibrary.PrintString` "Falied to Check out" false))
                    (:`OnMoveFinished`
                      (`self.Get Point`)
                      (`AITask_MoveTo.AIMoveTo` (`AIBlueprintHelperLibrary.GetAIController` self) (`KismetMathLibrary.MakeVector` (.x (`SceneComponent.K2_GetComponentLocation` (`Actor.RootComponent` (`/Game/Blueprints/FoodPlacementManager.Exit` (`self.DestinationManager`))))) (.y (`SceneComponent.K2_GetComponentLocation` (`Actor.RootComponent` (`/Game/Blueprints/FoodPlacementManager.Exit` (`self.DestinationManager`)))))) null -1.0 "Default" "Default" true false true
                        (:`OnMoveFinished`
                          (`/Game/Blueprints/FoodPlacementManager.ResetAiWaypoint` (`self.DestinationManager`) (`self.indexwaypoints`))
                          (`KismetSystemLibrary.PrintString` (`KismetStringLibrary.Conv_IntToString` (`self.indexwaypoints`)) false true (struct :`G` 0.66 :`B` 1.0 :`A` 1.0) 100.0)
                          (`KismetSystemLibrary.PrintString` "Resthappen" false true (struct :`G` 0.66 :`B` 1.0 :`A` 1.0) 100.0)
                          (`self.K2_DestroyActor` self))))))))))))))

(event `Move`
  (bind _indexwaypoints (`self.indexwaypoints`))
  ;[1 1 1] Comment
  (bind (_nextavablietableplacement _waypointindex) (`/Game/Blueprints/FoodPlacementManager.GetNextWaypoint` (`self.DestinationManager`)))
  (`/Engine/EditorBlueprintResources/StandardMacros.IsValid` _nextavablietableplacement
    (:`Is Valid`
      (set `self.indexwaypoints` _waypointindex)
      (bind _returnvalue (`KismetMathLibrary.MakeVector` (.x (`SceneComponent.K2_GetComponentLocation` (`/Game/Blueprints/TablePlaement.SphereWaypoint` _nextavablietableplacement))) (.y (`SceneComponent.K2_GetComponentLocation` (`/Game/Blueprints/TablePlaement.SphereWaypoint` _nextavablietableplacement))) 5.0))
      (`AITask_MoveTo.AIMoveTo` (`AIBlueprintHelperLibrary.GetAIController` self) _returnvalue null 0.1 "Default" "Default" true false true
        (:`OnRequestFailed`
          (`KismetSystemLibrary.PrintString` "Falied to move " true true (struct :`G` 0.66 :`B` 1.0 :`A` 1.0) 100.0))
        (:`OnMoveFinished`
          (`KismetSystemLibrary.PrintString` "Success " true true (struct :`G` 0.66 :`B` 1.0 :`A` 1.0) 100.0)
          (`self.PlayAnimMontage` "/Game/Blueprints/Charater/SitDown.SitDown")
          (if (or (== (`KismetMathLibrary.Conv_IntToByte` _indexwaypoints) 0) (== (`KismetMathLibrary.Conv_IntToByte` _indexwaypoints) 3) (== (`KismetMathLibrary.Conv_IntToByte` _indexwaypoints) 4) (== (`KismetMathLibrary.Conv_IntToByte` _indexwaypoints) 6) (== (`KismetMathLibrary.Conv_IntToByte` _indexwaypoints) 8) (== (`KismetMathLibrary.Conv_IntToByte` _indexwaypoints) 10) false)
            (`self.K2_SetActorLocationAndRotation` self _returnvalue (struct :`Yaw` -90.0) false true)
            (else
              (`self.K2_SetActorLocationAndRotation` self _returnvalue (struct :`Yaw` 90.0) false true)))
          (if (and (`/Game/Blueprints/TablePlaement.FoodonPlacemetn` _nextavablietableplacement) (> (`self.CurTime `) 0.0))
            (`KismetSystemLibrary.PrintString` "FOOD IS IS ON TABLE ")
            (if (not (`self.Ai _pay_cycle`))
              (set `self.Ai _pay_cycle` true)
              (bind _returnvalue_2 (`self.PlayAnimMontage` "/Game/Blueprints/Charater/standup.standup"))
              (`KismetSystemLibrary.Delay` _returnvalue_2)
              (`AITask_MoveTo.AIMoveTo` (`AIBlueprintHelperLibrary.GetAIController` self) (`KismetMathLibrary.MakeVector` (.x (`SceneComponent.K2_GetComponentLocation` (`Actor.RootComponent` (`/Game/Blueprints/FoodPlacementManager.Checkout` (`self.DestinationManager`))))) (.y (`SceneComponent.K2_GetComponentLocation` (`Actor.RootComponent` (`/Game/Blueprints/FoodPlacementManager.Checkout` (`self.DestinationManager`)))))) null 0.1 "Default" "Default" true false true
                (:`OnRequestFailed`
                  (`KismetSystemLibrary.PrintString` "Falied to Check out" false))
                (:`OnMoveFinished`
                  (`self.Get Point`)
                  (`AITask_MoveTo.AIMoveTo` (`AIBlueprintHelperLibrary.GetAIController` self) (`KismetMathLibrary.MakeVector` (.x (`SceneComponent.K2_GetComponentLocation` (`Actor.RootComponent` (`/Game/Blueprints/FoodPlacementManager.Exit` (`self.DestinationManager`))))) (.y (`SceneComponent.K2_GetComponentLocation` (`Actor.RootComponent` (`/Game/Blueprints/FoodPlacementManager.Exit` (`self.DestinationManager`)))))) null -1.0 "Default" "Default" true false true
                    (:`OnMoveFinished`
                      (`/Game/Blueprints/FoodPlacementManager.ResetAiWaypoint` (`self.DestinationManager`) (`self.indexwaypoints`))
                      (`KismetSystemLibrary.PrintString` (`KismetStringLibrary.Conv_IntToString` (`self.indexwaypoints`)) false true (struct :`G` 0.66 :`B` 1.0 :`A` 1.0) 100.0)
                      (`KismetSystemLibrary.PrintString` "Resthappen" false true (struct :`G` 0.66 :`B` 1.0 :`A` 1.0) 100.0)
                      (`self.K2_DestroyActor` self))))))))))
    (:`Is Not Valid`
      (`KismetSystemLibrary.PrintString` "not  valid waypoint" false true (struct :`G` 0.66 :`B` 1.0 :`A` 1.0) 100.0))))

(event `Get Point`
  ;[1 1 1] Points given
  (bind _asplayer_real (cast `/Game/Blueprints/Charater/PlayerReal` (`GameplayStatics.GetPlayerCharacter` 0)))
  (`/Game/Blueprints/Charater/PlayerReal.PointsUp` _asplayer_real))

(fn `TIMENPC`
  (bind _output_get (set `self.CurTime ` (- (`self.CurTime `) (`GameplayStatics.GetWorldDeltaSeconds`))))
  (bind _returnvalue (/ _output_get (`self.Maxtime`)))
  (if (<= _returnvalue 0.0)
    (set `self.CurTime ` 0.0))
  (bind _asnpcwait_timer (cast `/Game/UMG/NPCwaitTimer` (`WidgetComponent.GetUserWidgetObject` (`self.Waittime`))))
  (`ProgressBar.SetPercent` (`/Game/UMG/NPCwaitTimer.ProgressSlider` _asnpcwait_timer) _returnvalue))

(fn `UserConstructionScript`)