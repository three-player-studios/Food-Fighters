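; Interactable table with two food slots, where the player can set down held food or pick up food.
; Overlap events on Loc1 and Loc2 track where PlayerReal stands, and ObjectInteract calls that slot's function, with Loc1 taking priority.
; A valid slot reference is passed to the player's GrabItem; otherwise HeldFood is stored and snapped to that slot's mesh socket.
; The slot functions never clear their food references after a grab.
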(event `/Game/Blueprints/Interaction/I_Interact.Object_Interact`
  (if (`self.InLoc1`)
    (`self.FoodLoc1`)
    (elif (`self.InLoc2`)
      (`self.FoodLoc2`))))

(event `self.Loc1.OnComponentBeginOverlap`
  (params (OverlappedComponent :type "PrimitiveComponent Object Reference") (OtherActor :type "Actor Object Reference") (OtherComp :type "PrimitiveComponent Object Reference") (OtherBodyIndex :type Integer) (bFromSweep :type Boolean) (SweepResult :type "HitResult Structure (by ref)"))
  (cast `/Game/Blueprints/Charater/PlayerReal` OtherActor)
  (set `self.InLoc1` true))

(event `self.Loc1.OnComponentEndOverlap`
  (params (OverlappedComponent :type "PrimitiveComponent Object Reference") (OtherActor :type "Actor Object Reference") (OtherComp :type "PrimitiveComponent Object Reference") (OtherBodyIndex :type Integer))
  (cast `/Game/Blueprints/Charater/PlayerReal` OtherActor)
  (set `self.InLoc1` false))

(event `self.Loc2.OnComponentBeginOverlap`
  (params (OverlappedComponent :type "PrimitiveComponent Object Reference") (OtherActor :type "Actor Object Reference") (OtherComp :type "PrimitiveComponent Object Reference") (OtherBodyIndex :type Integer) (bFromSweep :type Boolean) (SweepResult :type "HitResult Structure (by ref)"))
  (cast `/Game/Blueprints/Charater/PlayerReal` OtherActor)
  (set `self.InLoc2` true))

(event `self.Loc2.OnComponentEndOverlap`
  (params (OverlappedComponent :type "PrimitiveComponent Object Reference") (OtherActor :type "Actor Object Reference") (OtherComp :type "PrimitiveComponent Object Reference") (OtherBodyIndex :type Integer))
  (cast `/Game/Blueprints/Charater/PlayerReal` OtherActor)
  (set `self.InLoc2` false))

(fn `FoodLoc1`
  (`/Engine/EditorBlueprintResources/StandardMacros.IsValid` (`self.Food1`)
    (:`Is Valid`
      (bind _asplayer_real (cast `/Game/Blueprints/Charater/PlayerReal` (`GameplayStatics.GetPlayerCharacter` 0)))
      (`/Game/Blueprints/Charater/PlayerReal.GrabItem` _asplayer_real (`self.Food1`)))
    (:`Is Not Valid`
      (bind _asplayer_real_2 (cast `/Game/Blueprints/Charater/PlayerReal` (`GameplayStatics.GetPlayerCharacter` 0)))
      (bind _output_get (set `self.Food1` (`FoodFightersCharacter.HeldFood` _asplayer_real_2)))
      (`self.K2_AttachToComponent` _output_get (`self.MyMesh`) "FOODBOX_1" "SnapToTarget" "SnapToTarget" "KeepWorld" true))))

(fn `FoodLoc2`
  (`/Engine/EditorBlueprintResources/StandardMacros.IsValid` (`self.Food2`)
    (:`Is Valid`
      (bind _asplayer_real (cast `/Game/Blueprints/Charater/PlayerReal` (`GameplayStatics.GetPlayerCharacter` 0)))
      (`/Game/Blueprints/Charater/PlayerReal.GrabItem` _asplayer_real (`self.Food2`)))
    (:`Is Not Valid`
      (bind _asplayer_real_2 (cast `/Game/Blueprints/Charater/PlayerReal` (`GameplayStatics.GetPlayerCharacter` 0)))
      (bind _output_get (set `self.Food2` (`FoodFightersCharacter.HeldFood` _asplayer_real_2)))
      (`self.K2_AttachToComponent` _output_get (`self.MyMesh`) "FOODBOX_2" "SnapToTarget" "SnapToTarget" "KeepWorld" true))))

(fn `UserConstructionScript`)