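; Food manager Blueprint that detects which food actor is on the table.
; Getfoodontable walks FoodTracker by index, testing the matching FoodR actor for overlap with Table.
; The first match is flagged true in FoodTracker, prints a debug "Hello" and is returned, regardless of its previous flag.
; The event graph, including the table's begin-overlap event, and the construction script contain no logic.
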(event `self.table.OnActorBeginOverlap`
  (params (OverlappedActor :type "Actor Object Reference") (OtherActor :type "Actor Object Reference")))

(fn `getfoodontable`
  (returns (Food :type "Food Object Reference"))
  (bind _foodtracker (`self.FoodTracker`))
  (for _index (range (`KismetArrayLibrary.Array_Length` _foodtracker))
    (bind _output (`|GetArrayItem` (`self.FoodR`) _index))
    (if (`self.IsOverlappingActor` _output (`self.table`))
      (`KismetArrayLibrary.Array_Set` _foodtracker _index true)
      (`KismetSystemLibrary.PrintString` "Hello")
      (return _output))))

(fn `UserConstructionScript`)