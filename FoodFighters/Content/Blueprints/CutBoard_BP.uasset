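; Cutting board actor where the player places a held food item or takes it back through ObjectInteract.
; Food transfers by class: the held item is removed and respawned on a mesh socket, or the board's item is destroyed and recreated on the player.
; While the player is cutting inside the box, Tick counts down a progress-bar widget and shows text at zero.
; Ending overlap resets the countdown; finishing leaves the food unchanged.
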(event `/Game/Blueprints/Interaction/I_Interact.Object_Interact`
  (`/Engine/EditorBlueprintResources/StandardMacros.IsValid` (`self.Food`)
    (:`Is Valid`
      (`self.RemoveFood`)
      (bind _asplayer_real (cast `/Game/Blueprints/Charater/PlayerReal` (`GameplayStatics.GetPlayerCharacter` 0)))
      (`/Game/Blueprints/Charater/PlayerReal.Createfood ` _asplayer_real (`GameplayStatics.GetObjectClass` (`self.Food`))))
    (:`Is Not Valid`
      (bind _asplayer_real_2 (cast `/Game/Blueprints/Charater/PlayerReal` (`GameplayStatics.GetPlayerCharacter` 0)))
      (`/Game/Blueprints/Charater/PlayerReal.RemoveFood` _asplayer_real_2)
      (`self.PlaceFood` (`GameplayStatics.GetObjectClass` (`FoodFightersCharacter.HeldFood` _asplayer_real_2))))))

(event `self.Box.OnComponentBeginOverlap`
  (params (OverlappedComponent :type "PrimitiveComponent Object Reference") (OtherActor :type "Actor Object Reference") (OtherComp :type "PrimitiveComponent Object Reference") (OtherBodyIndex :type Integer) (bFromSweep :type Boolean) (SweepResult :type "HitResult Structure (by ref)")))

(event `self.ReceiveActorOnClicked`
  (params (ButtonPressed :type "Key Structure")))

(event `self.ReceiveTick`
  (params (DeltaSeconds :type "Float (single-precision)"))
  (bind _asplayer_real (cast `/Game/Blueprints/Charater/PlayerReal` (`GameplayStatics.GetPlayerCharacter` 0)))
  (if (and (`/Game/Blueprints/Charater/PlayerReal.Cutting` _asplayer_real) (`PrimitiveComponent.IsOverlappingActor` (`self.Box`) _asplayer_real))
    (`self.Timer`)
    (if (<= (`self.CurTime `) 0.0)
      (`SceneComponent.SetVisibility` (`self.TextRender`) true false)
      (else
        (`SceneComponent.SetVisibility` (`self.TextRender`) false false)))))

(event `Key|LeftMouseButton`
  (params (Key :type "Key Structure")))

(event `self.ReceiveActorEndOverlap`
  (params (OtherActor :type "Actor Object Reference"))
  (set `self.CurTime ` 2.0))

(fn `PlaceFood`
  (params (NewParam :type "Food Class Reference"))
  (bind _returnvalue (`|SpawnActorFromClass` NewParam (`KismetMathLibrary.MakeTransform` (0.0 0.0 0.0)) "Undefined" "OverrideRootScale" null null))
  (`self.K2_AttachToComponent` _returnvalue (`self.Socketmesh`) "Cut Socket" "SnapToTarget" "KeepWorld" "KeepWorld" false)
  (set `self.Food` _returnvalue))

(fn `RemoveFood`
  (`/Engine/EditorBlueprintResources/StandardMacros.IsValid` (`self.Food`)
    (:`Is Valid`
      (`self.K2_DestroyActor` (`self.Food`)))))

(fn `Timer`
  (bind _output_get (set `self.CurTime ` (- (`self.CurTime `) (`GameplayStatics.GetWorldDeltaSeconds`))))
  (bind _returnvalue (/ _output_get (`self.MaxTime `)))
  (if (<= _returnvalue 0.0)
    _
    (else
      _))
  (bind _ascut_bar_timer (cast `/Game/UMG/CutBarTimer` (`WidgetComponent.GetUserWidgetObject` (`self.CutBar`))))
  (`ProgressBar.SetPercent` (`/Game/UMG/CutBarTimer.ProgressBar_97` _ascut_bar_timer) _returnvalue))

(fn `UserConstructionScript`)