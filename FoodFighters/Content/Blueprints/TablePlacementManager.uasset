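; TablePlacementManager hands out table placement waypoints, each paired with a target point, apparently for AI.
; GetNextWaypoint finds the first free slot in the WaypointTracker boolean array, marks it taken and returns the entries at that index from both waypoint arrays.
; ResetAiWaypoint runs the same free-slot search but writes the default false, so it returns that pair without releasing any taken slot.
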(event `self.ReceiveBeginPlay`)

(fn `GetNextWaypoint`
  (returns (NextAvablieTableplacement :type "/Game/Blueprints/TablePlaement Object Reference") (NextAvablieTarget :type "TargetPoint Object Reference"))
  (bind _waypointtracker (`self.WaypointTracker`))
  (for _index (range (`KismetArrayLibrary.Array_Length` _waypointtracker))
    (if (not (`|GetArrayItem` _waypointtracker _index))
      (`KismetSystemLibrary.PrintString` "Foundwaypoint")
      (`KismetArrayLibrary.Array_Set` _waypointtracker _index true)
      (return (`|GetArrayItem` (`self.Waypoints`) _index) (`|GetArrayItem` (`self.Waypointstargetpoint`) _index)))))

(fn `ResetAiWaypoint`
  (returns (NextAvablieTableplacement :type "/Game/Blueprints/TablePlaement Object Reference") (NextAvablieTarget :type "TargetPoint Object Reference"))
  (bind _waypointtracker (`self.WaypointTracker`))
  (for _index (range (`KismetArrayLibrary.Array_Length` _waypointtracker))
    (if (not (`|GetArrayItem` _waypointtracker _index))
      (`KismetSystemLibrary.PrintString` "Reset")
      (`KismetArrayLibrary.Array_Set` _waypointtracker _index)
      (return (`|GetArrayItem` (`self.Waypoints`) _index) (`|GetArrayItem` (`self.Waypointstargetpoint`) _index)))))

(fn `UserConstructionScript`)